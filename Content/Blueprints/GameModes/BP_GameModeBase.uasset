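; Game mode Blueprint that handles the start and end screens of a match and displays the player's score.
; GameStart creates the start widget with the start delay, and GameOver creates the end widget with whether the player won.
; BeginPlay and Tick share a debug PrintString of the player score, using the frame's delta time as duration so it reads as a live counter.
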(event `self.GameStart`
  ;[1 1 1] GameStartWidget
  (bind _returnvalue (`|CreateWidget` "/Game/Blueprints/Widgets/WBP_GameStart.WBP_GameStart_C"))
  (`/Game/Blueprints/Widgets/WBP_GameStart.SetStartDelay` _returnvalue (`self.StartDelay`))
  (`UserWidget.AddToViewport` _returnvalue 0))

(event `self.GameOver`
  (params (PlayerWon :type Boolean))
  ;[1 1 1] GameOverWidget
  (bind _returnvalue (`|CreateWidget` "/Game/Blueprints/Widgets/WBP_GameEnd.WBP_GameEnd_C"))
  (`/Game/Blueprints/Widgets/WBP_GameEnd.SetPlayerWon` _returnvalue PlayerWon)
  (`UserWidget.AddToViewport` _returnvalue 0))

(event `self.ReceiveBeginPlay`
  ;[1 1 1] PlayerScoring
  (`KismetSystemLibrary.PrintString` (`KismetStringLibrary.Conv_IntToString` (`self.ScorePlayer`)) true true (struct :`G` 0.66 :`B` 1.0 :`A` 1.0) (stale `self.ReceiveTick` DeltaSeconds) :!label _label))

(event `self.ReceiveTick`
  (params (DeltaSeconds :type "Float (single-precision)"))
  ;[1 1 1] PlayerScoring
  (goto _label))

(fn `UserConstructionScript`)